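; BP_PlayerController is the FPS player controller, and it toggles the pause menu.
; Completing IA_Menu drives a FlipFlop that either pauses, creates a fresh WBP_Menu, shows the cursor and focuses the menu in Game and UI input, or reverses this to game-only input.
; The menu's MenuClosed event re-enters the same FlipFlop, keeping toggle state in sync when the widget closes itself.
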(event Custom|MenuClosed_事件
  (Utilities|FlowControl|FlipFlop
    (:A
      (Game|SetGamePaused true)
      (bind _returnvalue (UserInterface|CreateWidget "/Game/FPS/Widget/WBP_Menu.WBP_Menu_C"))
      (bind _output_get (Variables|Default|SetMenu _returnvalue))
      (EventDispatchers|AssignMenuClosed _output_get (delegate Custom|MenuClosed_事件))
      (UserInterface|Viewport|AddtoViewport _output_get 0)
      (Input|SetInputModeGameandUI self _output_get "DoNotLock" true false)
      (Variables|Default|SetbShowMouseCursor true))
    (:B
      (Game|SetGamePaused false)
      (Widget|RemovefromParent (Variables|Default|GetMenu))
      (Input|SetInputModeGameOnly self false)
      (Variables|Default|SetbShowMouseCursor false))))

(event Input|EnhancedActionEvents|EnhancedInputActionIA_Menu
  (params (ActionValue :type Boolean) (ElapsedSeconds :type Float%20%28double-precision%29) (TriggeredSeconds :type Float%20%28double-precision%29) (InputAction :type Input%20Action%20Object%20Reference :default "/Game/FPS/Input/Actions/IA_Menu.IA_Menu"))
  (:Completed
    (Utilities|FlowControl|FlipFlop
      (:A
        (Game|SetGamePaused true)
        (bind _returnvalue (UserInterface|CreateWidget "/Game/FPS/Widget/WBP_Menu.WBP_Menu_C"))
        (bind _output_get (Variables|Default|SetMenu _returnvalue))
        (EventDispatchers|AssignMenuClosed _output_get (delegate Custom|MenuClosed_事件))
        (UserInterface|Viewport|AddtoViewport _output_get 0)
        (Input|SetInputModeGameandUI self _output_get "DoNotLock" true false)
        (Variables|Default|SetbShowMouseCursor true))
      (:B
        (Game|SetGamePaused false)
        (Widget|RemovefromParent (Variables|Default|GetMenu))
        (Input|SetInputModeGameOnly self false)
        (Variables|Default|SetbShowMouseCursor false)))))

(event EventBeginPlay)

(event EventTick
  (params (DeltaSeconds :type Float%20%28single-precision%29)))

(fn ConstructionScript)