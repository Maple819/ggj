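; AC_RenderTarget is an actor component that paints its owner's world position as a filled circle on a render target each frame.
; Every Tick it clears the target, maps the owner's XY by WorldSize around a centred origin to pixel coordinates, and draws a 100-sided polygon through the Canvas.
; The circle's radius scales by Radius over WorldSize.
; The draw pass begins but never calls EndDrawCanvasToRenderTarget.
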(event EventBeginPlay)

(event EventTick
  (params (DeltaSeconds :type Float%20%28single-precision%29))
  (bind _returnvalue (Components|GetOwner))
  (bind _texture_render_target (Variables|Default|GetTexture%20Render%20Target))
  (bind _worldsize (Variables|Default|GetWorldSize))
  (bind _radius (Variables|Default|GetRadius))
  (bind _returnvalue_2 (Transformation|GetActorLocation _returnvalue))
  (bind _returnvalue_3 (/ _radius _worldsize))
  (bind _sizex (Variables|/Script/Engine.TextureRenderTarget2D|GetSizeX _texture_render_target))
  (bind _sizey (Variables|/Script/Engine.TextureRenderTarget2D|GetSizeY _texture_render_target))
  (bind _returnvalue_4 (Math|Conversions|ToFloat(Integer) _sizex))
  (bind _returnvalue_5 (Math|Conversions|ToFloat(Integer) _sizey))
  (bind _returnvalue_6 (Math|Vector2D|MakeVector2D _returnvalue_4 _returnvalue_5))
  (Rendering|ClearRenderTarget2D _texture_render_target (Variables|/Script/Engine.TextureRenderTarget2D|GetClearColor _texture_render_target))
  (bind _canvas (Rendering|BeginDrawCanvastoRenderTarget _texture_render_target))
  (Class|Canvas|DrawPolygon _canvas 0 (* (Math|Vector2D|MakeVector2D (+ (/ (.x _returnvalue_2) _worldsize) 0.5) (+ (/ (.y _returnvalue_2) _worldsize) 0.5)) _returnvalue_6) (* _returnvalue_6 (Math|Vector2D|MakeVector2D _returnvalue_3 _returnvalue_3)) 100 "(R=1.000000,G=1.000000,B=1.000000,A=1.000000)"))