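; Configurable bomb actor that explodes on an optional timer, on taking damage, or on touch from an actor outside its ignore list.
; Construction and BeginPlay apply a skeletal or static mesh, removing unset components, and BeginPlay plays any placement animation.
; Mesh hits and box overlaps share one detonation check.
; Blow fires the OnBlow dispatcher, applies radial damage, spawns particle and sound, removes meshes, and destroys the actor shortly after.
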(event OnComponentHit(Bomb_SkeletalMesh)
  (params (HitComponent :type Primitive%20Component%20Object%20Reference) (OtherActor :type Actor%20Object%20Reference) (OtherComp :type Primitive%20Component%20Object%20Reference) (NormalImpulse :type Vector :default "0, 0, 0") (Hit :type Hit%20Result%20Structure%20%28by%20ref%29))
  (Variables|Private|SetSetHittedActor OtherActor)
  (if (not (Utilities|Array|ContainsItem (Variables|DamageSettings|GetIgnoreActors) (Variables|Private|GetSetHittedActor)))
    (if (Variables|Detonationsettings|GetTouchDetonation)
      (Utilities|FlowControl|DoOnce false
        (:Completed
          (CallFunction|Blow))))))

(event OnComponentHit(Bomb_StaticMesh)
  (params (HitComponent :type Primitive%20Component%20Object%20Reference) (OtherActor :type Actor%20Object%20Reference) (OtherComp :type Primitive%20Component%20Object%20Reference) (NormalImpulse :type Vector :default "0, 0, 0") (Hit :type Hit%20Result%20Structure%20%28by%20ref%29))
  (Variables|Private|SetSetHittedActor OtherActor)
  (if (not (Utilities|Array|ContainsItem (Variables|DamageSettings|GetIgnoreActors) (Variables|Private|GetSetHittedActor)))
    (if (Variables|Detonationsettings|GetTouchDetonation)
      (Utilities|FlowControl|DoOnce false
        (:Completed
          (CallFunction|Blow))))))

(event OnComponentBeginOverlap(Box)
  (params (OverlappedComponent :type Primitive%20Component%20Object%20Reference) (OtherActor :type Actor%20Object%20Reference) (OtherComp :type Primitive%20Component%20Object%20Reference) (OtherBodyIndex :type Integer) (bFromSweep :type Boolean) (SweepResult :type Hit%20Result%20Structure%20%28by%20ref%29))
  (Variables|Private|SetSetHittedActor OtherActor)
  (if (not (Utilities|Array|ContainsItem (Variables|DamageSettings|GetIgnoreActors) (Variables|Private|GetSetHittedActor)))
    (if (Variables|Detonationsettings|GetTouchDetonation)
      (Utilities|FlowControl|DoOnce false
        (:Completed
          (CallFunction|Blow))))))

(event Custom|Blow
  (bind _bomb_skeletalmesh (Variables|Default|GetBomb_SkeletalMesh))
  (bind _bomb_staticmesh (Variables|Default|GetBomb_StaticMesh))
  (Default|CallOnBlow)
  (Game|Damage|ApplyRadialDamage (Variables|DamageSettings|GetDamage) (Transformation|GetActorLocation) (Variables|DamageSettings|GetRadius) (Variables|DamageSettings|GetDamageTypeClass) (Variables|DamageSettings|GetIgnoreActors) (Components|GetOwner) 0 (Variables|DamageSettings|GetDoFullDamage) "ECC_Visibility")
  (Effects|SpawnEmitteratLocation (Variables|Visual|GetExplositonParticle) (Transformation|GetActorLocation))
  (Audio|SpawnSoundatLocation (Variables|Visual|GetSoundExplosion) (Transformation|GetActorLocation) "0, 0, 0" 1.0 1.0 0.0 0 0)
  (Utilities|FlowControl|Sequence
    (:then_0
      (Utilities|FlowControl|Delay 0.2)
      (Actor|DestroyActor))
    (:then_1
      (Utilities|IsValid _bomb_skeletalmesh
        (:Is%20Valid
          (Components|DestroyComponent _bomb_skeletalmesh))))
    (:then_2
      (Utilities|IsValid _bomb_staticmesh
        (:Is%20Valid
          (Components|DestroyComponent _bomb_staticmesh))))))

(event EventBeginPlay
  (|InitializationMesh)
  (|PlayPlaceBombAnimation)
  (Utilities|Array|Add (Variables|DamageSettings|GetIgnoreActors) self)
  (if (Variables|Detonationsettings|GetUseTimer)
    (Utilities|FlowControl|Delay (Variables|Detonationsettings|GetTimeForExplosion))
    (CallFunction|Blow)))

(event Game|Damage|EventAnyDamage
  (params (Damage :type Float%20%28single-precision%29) (DamageType :type Damage%20Type%20Object%20Reference) (InstigatedBy :type Controller%20Object%20Reference) (DamageCauser :type Actor%20Object%20Reference))
  (if (Variables|Detonationsettings|GetExplodesIfDamaged)
    (Utilities|FlowControl|DoOnce false
      (:Completed
        (CallFunction|Blow)))))

(fn ConstructionScript
  (|InitializationMesh))